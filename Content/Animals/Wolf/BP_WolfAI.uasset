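; Wolf AI Blueprint that computes four-legged foot IK data for ground placement.
; IKLogic, not called within this Blueprint, line-traces below each hand and foot socket from a capsule-derived height.
; IKSetup writes effector, normal and hit by reference per limb, zeroing alpha on a miss.
; Front and back pairs each keep the larger-magnitude hip offset, with optional debug drawing.
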(event EventBeginPlay
  (|CallParentFunction))

(event Collision|EventActorBeginOverlap
  (params (OtherActor :type Actor%20Object%20Reference)))

(event EventTick
  (params (DeltaSeconds :type Float%20%28single-precision%29)))

(fn ConstructionScript
  (|CallParentFunction)
  (Variables|IKSetup|SetIKRootOffset (/ (Variables|/Script/Engine.CapsuleComponent|GetCapsuleHalfHeight (Variables|Default|GetCapsuleComponent)) 2.0)))

(fn IKLogic
  (params (Disable :type Boolean) (Debug :type Boolean))
  (bind _mesh (Variables|Character|GetMesh))
  (if (not Disable)
    (bind _hipoffset (CallFunction|IKSetup Debug "R-Hand" (Variables|IKSetup|GetIK-EL-FrontRight) (Variables|IKSetup|GetIK-N-FrontRight) (Variables|IKSetup|GetIK-Hit-FrontRight) (Variables|IKSetup|GetIK-Alpha-FrontRight)))
    (bind _hipoffset_2 (CallFunction|IKSetup Debug "L-Hand" (Variables|IKSetup|GetIK-EL-FrontLeft) (Variables|IKSetup|GetIK-N-FrontLeft) (Variables|IKSetup|GetIK-Hit-FrontLeft) (Variables|IKSetup|GetIK-Alpha-FrontLeft)))
    (bind _value (CallFunction|IKChooseHipOffset _hipoffset _hipoffset_2))
    (Variables|IKSetup|SetIK-HipOffset-Front _value)
    (bind _hipoffset_3 (CallFunction|IKSetup Debug "R-Foot" (Variables|IKSetup|GetIK-EL-BackRight) (Variables|IKSetup|GetIK-N-BackRight) (Variables|IKSetup|GetIK-Hit-BackRight) (Variables|IKSetup|GetIK-Alpha-BackRight)))
    (bind _hipoffset_4 (CallFunction|IKSetup Debug "L-Foot" (Variables|IKSetup|GetIK-EL-BackLeft) (Variables|IKSetup|GetIK-N-BackLeft) (Variables|IKSetup|GetIK-Hit-BackLeft) (Variables|IKSetup|GetIK-Alpha-BackLeft)))
    (bind _value_2 (CallFunction|IKChooseHipOffset _hipoffset_3 _hipoffset_4))
    (Variables|IKSetup|SetIK-HipOffset-Back _value_2)
    (if Debug
      (Rendering|Debug|DrawDebugBox (Transformation|GetSocketLocation _mesh "Pelvis") "10.000000,10.000000,10.000000" "(R=0.000000,G=1.000000,B=0.049490,A=1.000000)" "0, 0, 0" 0.0 1.0)
      (Rendering|Debug|DrawDebugBox (Transformation|GetSocketLocation _mesh "Spine") "10.000000,10.000000,10.000000" "(R=0.987921,G=1.000000,B=0.000000,A=1.000000)" "0, 0, 0" 0.0 1.0)
      (Rendering|Debug|DrawDebugBox (Transformation|GetSocketLocation _mesh "Spine1") "10.000000,10.000000,10.000000" "(R=1.000000,G=0.550111,B=0.000000,A=1.000000)" "0, 0, 0" 0.0 1.0)
      (Rendering|Debug|DrawDebugBox (Transformation|GetSocketLocation _mesh "Spine2") "10.000000,10.000000,10.000000" "(R=1.000000,G=0.000000,B=0.027873,A=1.000000)" "0, 0, 0" 0.0 1.0))))

(fn IKFootTrace
  (params (Debug :type Boolean) (SocketName :type Name) (Trace%20Distance :type Float%20%28single-precision%29))
  (bind _returnvalue (Transformation|GetActorLocation))
  (bind _mesh (Variables|Character|GetMesh))
  (bind _ikrootoffset (Variables|IKSetup|GetIKRootOffset))
  (bind _returnvalue_2 (Transformation|GetSocketLocation _mesh SocketName))
  (bind (_x _y) (Math|Vector|BreakVector _returnvalue_2))
  (if Debug
    (Rendering|Debug|DrawDebugBox _returnvalue_2 "4.000000,4.000000,4.000000" "(R=1.000000,G=0.000000,B=0.000000,A=1.000000)" "0, 0, 0" 0.0 1.0)
    (LocalVariables|SetTrace%20Debug "ForOneFrame")
    (else
      (LocalVariables|SetTrace%20Debug "None")))
  (bind (_outhit _returnvalue_3) (Collision|LineTraceByChannel (Math|Vector|MakeVector _x _y (- (.z _returnvalue) _ikrootoffset)) (Math|Vector|MakeVector _x _y (- (.z _returnvalue) Trace%20Distance)) "TraceTypeQuery1" false 0 (LocalVariables|GetTrace%20Debug)))
  (if Debug
    (Rendering|Debug|DrawDebugSphere (.location _outhit) 1e+01 5 "(R=0.000000,G=0.016063,B=1.000000,A=1.000000)" 0.0 1.0))
  (return _returnvalue_3 (.impactpoint _outhit) (.normal _outhit) (Math|Float|SelectFloat (* (- (- (.z _returnvalue) (* _ikrootoffset 2.0)) (.Z (Math|Vector|BreakVector (.impactpoint _outhit)))) -1.0) 0.0 _returnvalue_3)))

(fn IKChooseHipOffset
  (params (Right :type Float%20%28single-precision%29) (Left :type Float%20%28single-precision%29))
  (return (Math|Float|SelectFloat Right Left (>= (Math|Float|Absolute(Float) Right) (Math|Float|Absolute(Float) Left)))))

(fn IKSetup
  (params (Debug :type Boolean) (Socket%20Name :type Name) (Effector%20Location :type Vector%20%28by%20ref%29) (Normal :type Vector%20%28by%20ref%29) (Hit :type Boolean) (Alpha :type Float%20%28single-precision%29%20%28by%20ref%29))
  (bind (_hit _effectorlocator _normal _hipoffset) (CallFunction|IKFootTrace Debug Socket%20Name (Variables|IKSetup|GetIKTraceDistance)))
  (|SetBy-RefVar Effector%20Location (+ _effectorlocator "0, 0,6.000000"))
  (|SetBy-RefVar Normal _normal)
  (|SetBy-RefVar Hit _hit)
  (if _hit
    _
    (else
      (|SetBy-RefVar Alpha 0.0)))
  (return _hipoffset))