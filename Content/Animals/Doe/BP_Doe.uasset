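; BP_Doe is a doe animal character that inherits its setup from a parent and adds a secondary attack.
; SecondaryAttack sphere-traces from just ahead of the AttackSocket2 mesh socket back along the forward vector, with debug drawing and a debug print.
; Hitting a BP_CharacterBase spawns blood, applies SecondaryAttackDamage and clears HasSecondaryAttack.
; The damage call passes the hit character, not the doe, as Sender.
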(event EventBeginPlay
  (|CallParentFunction))

(event Collision|EventActorBeginOverlap
  (params (OtherActor :type Actor%20Object%20Reference)))

(event EventTick
  (params (DeltaSeconds :type Float%20%28single-precision%29)))

(event EventSecondaryAttack
  (params (Target :type Actor%20Object%20Reference))
  (bind _returnvalue (Transformation|GetActorForwardVector))
  (bind _mesh (Variables|Character|GetMesh))
  (bind _returnvalue_2 (Transformation|GetSocketLocation _mesh "AttackSocket2"))
  (bind _returnvalue_3 (* _returnvalue -8e+01))
  (bind _returnvalue_4 (* _returnvalue 5e+01))
  (bind _returnvalue_5 (+ _returnvalue_4 _returnvalue_2))
  (bind _returnvalue_6 (+ _returnvalue_3 _returnvalue_5))
  (Development|PrintString "ExectureSecAttack")
  (bind _outhit (Collision|SphereTraceByChannel _returnvalue_5 (Math|Vector|MakeVector (.x _returnvalue_6) (.y _returnvalue_6) (.z _returnvalue_6)) 6e+01 "TraceTypeQuery4" false (Utilities|Array|MakeArray self) "ForDuration"))
  (bind _asbp_character_base (Utilities|Casting|CastToBP_CharacterBase (.HitActor (Collision|BreakHitResult _outhit))))
  (CallFunction|SpawnBloodatLocation (.Location (Collision|BreakHitResult _outhit)))
  (Default|GetDamage _asbp_character_base (Variables|Default|GetSecondaryAttackDamage) _asbp_character_base (.ImpactPoint (Collision|BreakHitResult _outhit)))
  (Variables|Default|SetHasSecondaryAttack false))

(fn ConstructionScript
  (|CallParentFunction))