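; Friendly wolf-boar animal Blueprint that extends its parent with a telegraphed charge as a secondary attack.
; SecondaryAttack holds a threatening state briefly, then enables Sphere overlaps, boosts walk speed and AI-moves to the target's location at that moment, retrying once on failure.
; The sphere damages any BP_CharacterBase it overlaps until the move ends.
; CanDoSecondaryAttack adds a timer-based cooldown to the parent's check, re-armed by ResetSecondaryAttack.
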(event OnComponentBeginOverlap(Sphere)
  (params (OverlappedComponent :type Primitive%20Component%20Object%20Reference) (OtherActor :type Actor%20Object%20Reference) (OtherComp :type Primitive%20Component%20Object%20Reference) (OtherBodyIndex :type Integer) (bFromSweep :type Boolean) (SweepResult :type Hit%20Result%20Structure%20%28by%20ref%29))
  (bind _asbp_character_base (Utilities|Casting|CastToBP_CharacterBase OtherActor))
  (Development|PrintString (Utilities|GetDisplayName OtherComp))
  (Default|GetDamage _asbp_character_base 5e+01 self "0, 0, 0"))

(event EventBeginPlay
  (|CallParentFunction))

(event Collision|EventActorBeginOverlap
  (params (OtherActor :type Actor%20Object%20Reference)))

(event EventSecondaryAttack
  (params (Target :type Actor%20Object%20Reference))
  (bind _returnvalue (Transformation|GetActorLocation Target))
  (bind _self self)
  (bind _returnvalue_2 (AI|GetAIController _self))
  ;[1 1 1] SecondaryAttack
  (Development|PrintString (Utilities|GetDisplayName Target) true true "(R=1.000000,G=0.682395,B=0.000000,A=1.000000)")
  (Variables|Default|SetIsThreatening true)
  (Utilities|FlowControl|Delay 2.2)
  (Variables|Default|SetIsThreatening false)
  (Variables|/Script/Engine.PrimitiveComponent|SetbGenerateOverlapEvents (Variables|Default|GetSphere) true)
  (Variables|/Script/Engine.CharacterMovementComponent|SetMaxWalkSpeed (Variables|Character|GetCharacterMovement) (+ (Variables|Default|GetRunSpeed) 1e+03))
  (AI|AIMoveTo _returnvalue_2 _returnvalue 0 -1.0 "Default" "Default" true true
    (:OnRequestFailed
      (AI|AIMoveTo _returnvalue_2 _returnvalue 0 -1.0 "Default" "Default" true true
        (:OnRequestFailed
          _)
        (:OnMoveFinished
          _)))
    (:OnMoveFinished
      _))
  (Variables|/Script/Engine.PrimitiveComponent|SetbGenerateOverlapEvents (Variables|Default|GetSphere) false))

(fn ConstructionScript
  (|CallParentFunction))

(fn CanDoSecondaryAttack
  (if (|CallParentFunction)
    (bind _returnvalue (Utilities|Time|SetTimerbyFunctionName 0 "ResetSecondaryAttack" (Variables|Default|GetSecondaryAttackCooldownTime)))
    (Variables|Default|SetSecondaryAttackTimer _returnvalue)
    (Variables|Default|SetHasSecondaryAttack false)
    (return true)
    (else
      (return false))))

(fn ResetSecondaryAttack
  (Variables|Default|SetHasSecondaryAttack true)
  (Utilities|Time|ClearandInvalidateTimerbyHandle (Variables|Default|GetSecondaryAttackTimer)))