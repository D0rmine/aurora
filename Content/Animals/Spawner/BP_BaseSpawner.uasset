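; Base animal spawner that scatters a set number of animals on the navmesh around a box volume.
; The construction script sizes the box, then SpawnAnimals picks random points in it and queries the first RecastNavMesh for a navigable location near each.
; AnimalType adds each animal as a child actor component at that relative location with random yaw.
; Failed navmesh lookups print a warning.
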(event EventBeginPlay)

(event Collision|EventActorBeginOverlap
  (params (OtherActor :type Actor%20Object%20Reference)))

(event EventTick
  (params (DeltaSeconds :type Float%20%28single-precision%29)))

(fn ConstructionScript
  (Components|Box|SetBoxExtent (Variables|Default|GetBox) (Variables|Default|GetBoxExtend) true)
  (switch int 0
    (:Default
      (CallFunction|SpawnAnimals))))

(fn SpawnAnimals
  (bind _box (Variables|Default|GetBox))
  (bind _outactors (Actor|GetAllActorsOfClass "/Script/Engine.RecastNavMesh"))
  (for _index (range 1 (Variables|Default|GetNumberOfAnimals))
    (if (.ReturnValue (Class|NavigationSystem|GetRandomPointinNavigableRadius (Utilities|Array|Get(acopy) _outactors) (+ (Transformation|GetActorLocation) (Math|Random|RandomPointinBoundingBox (Variables|/Script/Engine.SceneComponent|GetRelativeLocation _box) (Variables|/Script/Engine.BoxComponent|GetBoxExtent _box))) 1e+03 (Utilities|Array|Get(acopy) _outactors)))
      (bind _output_get (Variables|Default|SetDebug_Tmp (Math|Vector|MakeVector (.x (.RandomLocation (Class|NavigationSystem|GetRandomPointinNavigableRadius (Utilities|Array|Get(acopy) _outactors) (+ (Transformation|GetActorLocation) (Math|Random|RandomPointinBoundingBox (Variables|/Script/Engine.SceneComponent|GetRelativeLocation _box) (Variables|/Script/Engine.BoxComponent|GetBoxExtent _box))) 1e+03 (Utilities|Array|Get(acopy) _outactors)))) (.y (.RandomLocation (Class|NavigationSystem|GetRandomPointinNavigableRadius (Utilities|Array|Get(acopy) _outactors) (+ (Transformation|GetActorLocation) (Math|Random|RandomPointinBoundingBox (Variables|/Script/Engine.SceneComponent|GetRelativeLocation _box) (Variables|/Script/Engine.BoxComponent|GetBoxExtent _box))) 1e+03 (Utilities|Array|Get(acopy) _outactors)))) (+ (.z (.RandomLocation (Class|NavigationSystem|GetRandomPointinNavigableRadius (Utilities|Array|Get(acopy) _outactors) (+ (Transformation|GetActorLocation) (Math|Random|RandomPointinBoundingBox (Variables|/Script/Engine.SceneComponent|GetRelativeLocation _box) (Variables|/Script/Engine.BoxComponent|GetBoxExtent _box))) 1e+03 (Utilities|Array|Get(acopy) _outactors)))) 0.0))))
      (CallFunction|AnimalType (- _output_get (Transformation|GetActorLocation)) (Math|Rotator|MakeRotator 0.0 0.0 (Math|Random|RandomFloatinRange 0.0 3.6e+02)))
      (else
        (Development|PrintString "Spawner : Failed to find location in nav")))))

(fn AnimalType
  (params (Location :type Vector) (Rotation :type Rotator))
  (AddComponent|AddChildActorComponent false (Math|Transform|MakeTransform Location Rotation "1,1,1")))