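; Fox animal Blueprint, a child class that leaves most behavior to its parent.
; Its GetDamage override runs the parent damage logic, then switches AnimalAttitude to another enum state when Health drops below a quarter of FullHealth.
; The parent's result is returned only on that low-health branch.
; BeginPlay and the construction script just call the parent, and the overlap event is empty.
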(event EventBeginPlay
  (|CallParentFunction))

(event Collision|EventActorBeginOverlap
  (params (OtherActor :type Actor%20Object%20Reference)))

(fn ConstructionScript
  (|CallParentFunction))

(fn GetDamage
  (params (Damage :type Float%20%28single-precision%29) (Sender :type Actor%20Object%20Reference) (HitLocation :type Vector :default "0, 0, 0"))
  (bind _gotkilled (|CallParentFunction Damage Sender HitLocation))
  (if (< (Variables|Default|GetHealth) (/ (Variables|Default|GetFullHealth) 4.0))
    (Variables|Default|SetAnimalAttitude "NewEnumerator2")
    (return _gotkilled)))